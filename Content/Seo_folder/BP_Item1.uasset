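; BP_Item1 is a spinning item pickup for BP_PlayerSum.
; A timeline started on Tick drives the yaw of its Box component.
; On Box overlap with a BP_PlayerSum it queries CanGetItem, and a false result leads to pickup.
; Pickup fires the RespawnItem dispatcher with location and self, plays the ItemGet sound at the player, then destroys the actor.
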(event OnComponentBeginOverlap(Box)
  (params (OverlappedComponent :type Primitive%20Component%20Object%20Reference) (OtherActor :type Actor%20Object%20Reference) (OtherComp :type Primitive%20Component%20Object%20Reference) (OtherBodyIndex :type Integer) (bFromSweep :type Boolean) (SweepResult :type Hit%20Result%20Structure%20%28by%20ref%29))
  (bind _asbp_player_sum (Utilities|Casting|CastToBP_PlayerSum OtherActor))
  (bind _dont_get (Default|CanGetItem _asbp_player_sum))
  (if (not _dont_get)
    (Default|CallRespawnItem (Transformation|GetActorLocation) self)
    (Audio|PlaySoundatLocation "/Game/sound/ItemGet.ItemGet" (Transformation|GetActorLocation _asbp_player_sum) "0, 0, 0" 1.0 1.0 0.0 0 0 0 0)
    (Actor|DestroyActor)))

(event EventBeginPlay
  (Variables|Default|SetItem_Location (Transformation|GetActorLocation)))

(event Collision|EventActorBeginOverlap
  (params (OtherActor :type Actor%20Object%20Reference)))

(event EventTick
  (params (DeltaSeconds :type Float%20%28single-precision%29))
  (bind _angle (Timeline|타임라인 Play)
    (:Update
      (Transformation|SetRelativeRotation (Variables|Default|GetBox) (Math|Rotator|MakeRotator 0.0 0.0 (* _angle 1.8e+02)) false false))))

(fn ConstructionScript)