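; Player character Blueprint with a two-slot random item system, shown as icons on a HUD widget.
; CanGetItem fills an empty slot with a random ID; keys 1 and 2 trigger that slot's skill: grenade, slow-fall feather, gum, grab or kimchi screen overlay.
; Used items are cleared, with slot 2 shifting into an empty slot 1, while CanUsed gates feather and grab consumption.
; Landing restores gravity and removes the feather.
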(event OnComponentBeginOverlap(Sphere)
  (params (OverlappedComponent :type Primitive%20Component%20Object%20Reference) (OtherActor :type Actor%20Object%20Reference) (OtherComp :type Primitive%20Component%20Object%20Reference) (OtherBodyIndex :type Integer) (bFromSweep :type Boolean) (SweepResult :type Hit%20Result%20Structure%20%28by%20ref%29))
  ;[1 1 1] 그랩
  (Variables|Default|Setcan_grap true))

(event OnComponentEndOverlap(Sphere)
  (params (OverlappedComponent :type Primitive%20Component%20Object%20Reference) (OtherActor :type Actor%20Object%20Reference) (OtherComp :type Primitive%20Component%20Object%20Reference) (OtherBodyIndex :type Integer))
  ;[1 1 1] 그랩
  (Variables|Default|Setcan_grap false))

(event Custom|Item_Update
  (bind _item_list (Variables|Default|GetItem_list))
  ;[1 1 1] Item 화면 갱신
  (CallFunction|FindIndex (Utilities|Array|Get(acopy) _item_list) (Utilities|Array|Get(acopy) _item_list 1)))

(event Custom|Use_Item
  (params (Key :type Integer))
  (bind _item_list (Variables|Default|GetItem_list))
  (bind _item_list_2 (Variables|Default|GetItem_list))
  ;[1 1 1] 아이템 사용시 해당 인덱스 스킬 제거
  (switch int Key
    (:1
      (Variables|Default|Setproto_slot1 (Utilities|Array|Get(acopy) _item_list_2))
      (Utilities|Array|SetArrayElem _item_list 0 0)
      (CallFunction|ItemUpdate)
      (CallFunction|ChangeIndex))
    (:2
      (Variables|Default|Setproto_slot2 (Utilities|Array|Get(acopy) _item_list_2 1))
      (Utilities|Array|SetArrayElem _item_list 1 0)
      (CallFunction|ItemUpdate)))
  (Variables|Default|SetCan_Used false))

(event Custom|change_index
  (bind _item_list (Variables|Default|GetItem_list))
  ;[1 1 1] 1번 사용시 2번스킬을 1번으로 옮김
  (if (== (Utilities|Array|Get(acopy) _item_list) 0)
    (Utilities|Array|SetArrayElem _item_list 0 (Utilities|Array|Get(acopy) (Variables|Default|GetItem_list) 1))
    (Utilities|Array|SetArrayElem _item_list 1 0)
    (CallFunction|ItemUpdate)))

(event Custom|Use_Kimchi
  ;[1 1 1] 김치
  (bind _returnvalue (UserInterface|CreateWidget "/Game/Seo_folder/WB_Gimchi.WB_Gimchi_C"))
  (UserInterface|Viewport|AddtoViewport _returnvalue 0))

(event Custom|Use_Gum
  (bind _returnvalue (Transformation|GetActorLocation))
  ;[1 1 1] 껌
  (if (Variables|Default|Getcan_gum)
    (bind _outhit (Collision|LineTraceByChannel _returnvalue (- _returnvalue "0.000000,0.000000,1000.000000") "TraceTypeQuery1" false 0 "None"))
    (Game|SpawnActorfromClass "/Game/Seo_folder/BP_Gum.BP_Gum_C" (Math|Conversions|ToTransform(Vector) (.ImpactPoint (Collision|BreakHitResult _outhit))) "Undefined" "MultiplyWithRoot" 0 0)))

(event Custom|Use_Grap
  (bind _returnvalue (Game|GetPlayerCharacter 0))
  ;[1 1 1] 그랩
  (if (Variables|Default|Getcan_grap)
    (Variables|Default|SetCan_Used true)
    (Transformation|SetActorLocation (stale OnComponentBeginOverlap(Sphere) OtherActor) (+ (* (Transformation|GetActorForwardVector _returnvalue) 2e+01) (Transformation|GetActorLocation _returnvalue)) false false)))

(event Custom|Use_Boom
  ;[1 1 1] 수류탄
  (bind _returnvalue (Game|SpawnActorfromClass "/Game/BP_Item_Boom.BP_Item_Boom_C" (Math|Conversions|ToTransform(Vector) (Transformation|GetSocketLocation (Variables|Character|GetMesh) "thumb_01_r")) "Undefined" "MultiplyWithRoot" 0 0))
  (Physics|AddImpulse (Variables|/Game/BP_Item_Boom.BP_Item_Boom_C|GetSphere _returnvalue) (* 3e+03 (Math|Vector|GetForwardVector (Variables|Default|GetFollowCamera))) "None" false))

(event Custom|Use_Grate
  (bind _charactermovement (Variables|Character|GetCharacterMovement))
  (bind _returnvalue (AI|Components|NavMovement|IsFalling _charactermovement))
  ;[1 1 1] 깃털
  (if _returnvalue
    (bind _output_get (Variables|Default|SetIs_grate _returnvalue))
    (Variables|Default|SetCan_Used _output_get)
    (bind _returnvalue_2 (Game|SpawnActorfromClass "/Game/Seo_folder/BP_great.BP_great_C" (Math|Conversions|ToTransform(Vector) "0, 0, 0") "Undefined" "MultiplyWithRoot" 0 0))
    (Variables|Default|Setobject_grate _returnvalue_2)
    (Transformation|AttachComponentToComponent _returnvalue_2 (Variables|Character|GetMesh) "top_head" "KeepRelative" "KeepRelative" "KeepRelative" true)
    (Transformation|SetActorRotation _returnvalue_2)
    (Variables|/Script/Engine.CharacterMovementComponent|SetGravityScale (Variables|Character|GetCharacterMovement) (Variables|Default|Getdecrease_gravity))
    (else
      (Variables|Default|SetCan_Used false))))

(event Collision|EventActorBeginOverlap
  (params (OtherActor :type Actor%20Object%20Reference))
  ;[1 1 1] 땅에 닿으면
)

(event EventBeginPlay
  ;[1 1 1] 게임시작시 위젯 생성
  (Utilities|FlowControl|Sequence
    (:then_0
      (bind _returnvalue (UserInterface|CreateWidget "/Game/Seo_folder/WB_HUD.WB_HUD_C"))
      (UserInterface|Viewport|AddtoViewport _returnvalue 0)
      (Variables|Default|SetHUD _returnvalue)
      (Variables|Default|SetSlot_1 (Variables|/Game/Seo_folder/WB_HUD.WB_HUD_C|Getslot_1 _returnvalue))
      (Variables|Default|SetSlot_2 (Variables|/Game/Seo_folder/WB_HUD.WB_HUD_C|Getslot_2 _returnvalue)))
    (:then_1
      (Variables|Default|SetController_Index (Class|GameplayStatics|GetPlayerControllerID (Game|GetPlayerController 0))))))

(event EventOnLanded
  (params (Hit :type Hit%20Result%20Structure%20%28by%20ref%29))
  ;[1 1 1] 땅에 닿으면
  (Variables|/Script/Engine.CharacterMovementComponent|SetGravityScale (Variables|Character|GetCharacterMovement) (Variables|Default|Getdefalut_gravity))
  (Variables|Default|Setcan_gum true)
  (if (Variables|Default|GetIs_grate)
    (Variables|Default|SetIs_grate false)
    (Actor|DestroyActor (Variables|Default|Getobject_grate))))

(event Input|KeyboardEvents|DebugKey1
  (params (Key :type Key%20Structure :default "None") (ActionValue :type Input%20Action%20Value%20Structure))
  ;[1 1 1] 스킬 구현
  (:Pressed
    (bind _output_get (Variables|Default|Setproto_slot1 (Utilities|Array|Get(acopy) (Variables|Default|GetItem_list))))
    (switch int _output_get
      (:1
        (CallFunction|UseBoom)
        (CallFunction|UseItem 1 :!label _label))
      (:2
        (CallFunction|UseGrate)
        (if (Variables|Default|GetCan_Used) :!label _label_2
          (goto _label)))
      (:3
        (CallFunction|UseGum)
        (goto _label))
      (:5
        (CallFunction|UseGrap)
        (goto _label_2))
      (:7
        (CallFunction|UseKimchi)
        (goto _label)))))

(event Input|MouseEvents|DebugKeyLeftMouseButton
  (params (Key :type Key%20Structure :default "None") (ActionValue :type Input%20Action%20Value%20Structure))
  (:Pressed
    (CallFunction|UseBoom)))

(event Input|KeyboardEvents|DebugKey2
  (params (Key :type Key%20Structure :default "None") (ActionValue :type Input%20Action%20Value%20Structure))
  ;[1 1 1] 스킬 구현
  (:Pressed
    (bind _output_get (Variables|Default|Setproto_slot2 (Utilities|Array|Get(acopy) (Variables|Default|GetItem_list) 1)))
    (switch int _output_get
      (:1
        (CallFunction|UseBoom)
        (CallFunction|UseItem 2 :!label _label))
      (:2
        (CallFunction|UseGrate)
        (if (Variables|Default|GetCan_Used) :!label _label_2
          (goto _label)))
      (:3
        (CallFunction|UseGum)
        (goto _label))
      (:5
        (CallFunction|UseGrap)
        (goto _label_2))
      (:7
        (CallFunction|UseKimchi)
        (goto _label)))))

(fn ConstructionScript)

(fn FindIndex
  (params (item0 :type Integer) (item1 :type Integer))
  (bind _as텍스처_2d (Utilities|Casting|CastToTexture2D (Utilities|Array|Get(acopy) (Variables|Default|GetItem_Image) item0)))
  (Appearance|SetBrushfromTexture (Variables|Default|GetSlot_1) _as텍스처_2d false)
  (bind _as텍스처_2d_2 (Utilities|Casting|CastToTexture2D (Utilities|Array|Get(acopy) (Variables|Default|GetItem_Image) item1)))
  (Appearance|SetBrushfromTexture (Variables|Default|GetSlot_2) _as텍스처_2d_2 false))

(fn CanGetItem
  (bind _item_list (Variables|Default|GetItem_list))
  (bind _item_list_2 (Variables|Default|GetItem_list))
  (if (and (!= (Utilities|Array|Get(acopy) _item_list) 0) (!= (Utilities|Array|Get(acopy) _item_list 1) 0))
    (return true)
    (elif (== (Utilities|Array|Get(acopy) _item_list_2) 0)
      (Utilities|Array|SetArrayElem (Variables|Default|GetItem_list) 0 (Math|Random|RandomIntegerinRange 1 7))
      (CallFunction|ItemUpdate :!label _label)
      (elif (== (Utilities|Array|Get(acopy) _item_list_2 1) 0)
        (Utilities|Array|SetArrayElem (Variables|Default|GetItem_list) 1 (Math|Random|RandomIntegerinRange 1 7))
        (goto _label)))))

(fn 새함수)