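; BP_Gum is a gum trap actor that immobilizes a BP_Seo character on overlap.
; The Gum component's overlap requires a BP_PlayerController and acts only when the character's ControllerIndex differs from that controller's player ID.
; It disables movement, sets a timer to restore walking, then immediately destroys itself.
; The restore event lives on the destroyed gum, so that timer is at risk of never firing.
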(event OnComponentBeginOverlap(Gum)
  (params (OverlappedComponent :type Primitive%20Component%20Object%20Reference) (OtherActor :type Actor%20Object%20Reference) (OtherComp :type Primitive%20Component%20Object%20Reference) (OtherBodyIndex :type Integer) (bFromSweep :type Boolean) (SweepResult :type Hit%20Result%20Structure%20%28by%20ref%29))
  (bind _asbp_seo (Utilities|Casting|CastToBP_Seo OtherActor))
  (bind _as캐릭터 (Utilities|Casting|CastToCharacter OtherActor))
  (bind _asbp_player_controller (Utilities|Casting|CastToBP_PlayerController (Pawn|GetController _as캐릭터)))
  (if (!= (Variables|/Game/Seo_folder/BP_Seo.BP_Seo_C|GetController_Index _asbp_seo) (Class|GameplayStatics|GetPlayerControllerID _asbp_player_controller))
    (Pawn|Components|CharacterMovement|SetMovementMode (Variables|/Script/Engine.Character|GetCharacterMovement _as캐릭터) "MOVE_None" 0)
    (Utilities|Time|SetTimerbyEvent (delegate Custom|Enable%20Movement) 5.0)
    (Actor|DestroyActor)))

(event Custom|Enable%20Movement
  (Pawn|Components|CharacterMovement|SetMovementMode (Variables|/Script/Engine.Character|GetCharacterMovement (stale OnComponentBeginOverlap(Gum) _as캐릭터)) "MOVE_Walking" 0))

(event EventBeginPlay)

(event Collision|EventActorBeginOverlap
  (params (OtherActor :type Actor%20Object%20Reference)))

(event EventTick
  (params (DeltaSeconds :type Float%20%28single-precision%29)))

(fn ConstructionScript)