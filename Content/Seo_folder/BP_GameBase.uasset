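; BP_GameBase is a game mode that spawns the selected character and times each run.
; Its construction script sets DefaultPawnClass to Edward, Sam or Hanly from the choice stored in GameInstance_Select.
; GameStart records the start time; GameOver saves the elapsed time to the game instance, lowers the stored minimum if beaten, and opens GameResult_Level.
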(event Custom|GameOver
  (bind _as_game_instance_select (Variables|Default|GetAs%20Game%20Instance%20Select))
  (bind _as_game_instance_select_2 (Variables|Default|GetAs%20Game%20Instance%20Select))
  (bind _output_get (Variables|Default|SetEndGameTime (Math|DateTime|Now)))
  (Variables|/Game/UI/GameInstance_Select.GameInstance_Select_C|SetCurrentScoreTime (Variables|Default|GetAs%20Game%20Instance%20Select) (- _output_get (Variables|Default|GetStartGameTime)))
  (if (< (Variables|/Game/UI/GameInstance_Select.GameInstance_Select_C|GetCurrentScoreTime _as_game_instance_select) (Variables|/Game/UI/GameInstance_Select.GameInstance_Select_C|GetMinScoreTime _as_game_instance_select))
    (Variables|/Game/UI/GameInstance_Select.GameInstance_Select_C|SetMinScoreTime _as_game_instance_select_2 (Variables|/Game/UI/GameInstance_Select.GameInstance_Select_C|GetCurrentScoreTime _as_game_instance_select_2)))
  (Game|OpenLevel(byName) "GameResult_Level"))

(event Custom|GameStart
  (bind _output_get (Variables|Default|SetStartGameTime (Math|DateTime|Now)))
  (Development|PrintString (Utilities|String|ToString(Text) (Utilities|Text|FormatText "{hour}:{minute}:{second}" (Utilities|Text|ToText(Integer) (.Hour (Math|DateTime|BreakDateTime _output_get)) false true 2) (Utilities|Text|ToText(Integer) (.Minute (Math|DateTime|BreakDateTime _output_get)) false true 2) (Utilities|Text|ToText(Integer) (.Second (Math|DateTime|BreakDateTime _output_get)) false true 2)))))

(event EventBeginPlay
  (bind _asgame_instance_select (Utilities|Casting|CastToGameInstance_Select (Game|GetGameInstance)))
  (Variables|Default|SetAs%20Game%20Instance%20Select _asgame_instance_select))

(fn ConstructionScript
  (bind _asgame_instance_select (Utilities|Casting|CastToGameInstance_Select (Game|GetGameInstance)))
  (bind _output_get (Variables|Default|SetSelect%20Character (Variables|/Game/UI/GameInstance_Select.GameInstance_Select_C|GetSelect_Character _asgame_instance_select)))
  (switch Utilities|FlowControl|Switch|SwitchonCharacterType _output_get
    (:NewEnumerator0
      (Variables|Default|SetDefaultPawnClass "/Game/Character/BP_Edward.BP_Edward_C")
      (Development|PrintString "에드워드실행"))
    (:NewEnumerator1
      (Variables|Default|SetDefaultPawnClass "/Game/Character/BP_Sam.BP_Sam_C")
      (Development|PrintString "샘 실행"))
    (:NewEnumerator2
      (Variables|Default|SetDefaultPawnClass "/Game/Character/BP_Hanly.BP_Hanly_C")
      (Development|PrintString "핸리 실행"))))