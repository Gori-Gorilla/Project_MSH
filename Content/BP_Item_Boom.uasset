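; BP_Item_Boom is a timed bomb item actor that knocks nearby players away.
; Four seconds after BeginPlay it plays a boom sound, runs Explode and destroys itself.
; Explode sphere-overlaps BP_PlayerSum actors and applies an outward CharacterMovement impulse, scaled by their offset and ExplodePower, so farther players get pushed harder.
; A particle emitter spawns after DestroyActor but is immediately destroyed and deactivated.
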(event Custom|explode
  (bind _outactors (Collision|SphereOverlapActors (Transformation|GetActorLocation) (Variables|Default|GetSphere%20Radius) (Variables|Default|GetObject%20Types) "/Game/ThirdPerson/Blueprints/BP_PlayerSum.BP_PlayerSum_C"))
  (for _array_element _outactors
    (Physics|AddImpulse (Actor|GetComponentbyClass _array_element "/Script/Engine.CharacterMovementComponent") (* (- (Transformation|GetActorLocation _array_element) (Transformation|GetActorLocation)) (Variables|Default|GetExplode_Power)) false)))

(event EventBeginPlay
  (bind _returnvalue (Transformation|GetActorLocation))
  (Utilities|FlowControl|Delay 4.0)
  (Audio|PlaySoundatLocation "/Game/Seo_folder/sound/sound_boom.sound_boom" _returnvalue "0, 0, 0" 1.0 1.0 0.0 0 0 0 0)
  (CallFunction|Explode)
  (Actor|DestroyActor)
  (bind _returnvalue_2 (Effects|SpawnEmitteratLocation "/Engine/Tutorial/SubEditors/TutorialAssets/TutorialParticleSystem.TutorialParticleSystem" _returnvalue "0, 0, 0" "1.000000,1.000000,1.000000" true "AutoRelease"))
  (Components|DestroyComponent _returnvalue_2)
  (Components|Activation|Deactivate _returnvalue_2))

(event Collision|EventActorBeginOverlap
  (params (OtherActor :type Actor%20Object%20Reference)))

(event EventTick
  (params (DeltaSeconds :type Float%20%28single-precision%29)))

(fn ConstructionScript)