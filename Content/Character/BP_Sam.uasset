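; BP_Sam is the Sam character Blueprint, which assigns Sam's skill on BeginPlay and adds a landing shockwave after a drop.
; Tick records the location where each fall begins, using a flag so it is captured only once while airborne.
; On landing, a large enough height drop triggers the shockwave, while smaller drops just print the difference.
; The shockwave plays a sound and impulses overlapping AI characters away from Sam.
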(event Custom|shock_wave
  (CallFunction|EventSound "/Game/sound/Sam_shockwave.Sam_shockwave")
  (for _array_element (Collision|GetOverlappingActors (Variables|Default|Getshock%20wave_collider) "/Game/Character/AI/BP_AICharacter.BP_AICharacter_C" :!class /Script/Engine.PrimitiveComponent)
    (Physics|AddImpulse (Actor|GetComponentbyClass _array_element "/Script/Engine.CharacterMovementComponent") (* (- (Transformation|GetActorLocation _array_element) (Transformation|GetActorLocation)) 8e+03) false)))

(event EventBeginPlay
  (|CallParentFunction)
  (Default|SkillChange (Variables|Default|Getskill) "/Game/Image/skill_sam.skill_sam"))

(event Collision|EventActorBeginOverlap
  (params (OtherActor :type Actor%20Object%20Reference))
  (|CallParentFunction OtherActor) ; 지금 이 노드는 비활성 상태입니다. \n핀을 끌어서 다른 노드를 연결하면 활성화됩니다.
)

(event EventTick
  (params (DeltaSeconds :type Float%20%28single-precision%29))
  (|CallParentFunction DeltaSeconds)
  (if (AI|Components|NavMovement|IsFalling (Variables|Character|GetCharacterMovement))
    (if (not (Variables|Default|Getcal_z))
      (Variables|Default|Setcal_z true)
      (Variables|Default|Setbefore_z (Transformation|GetActorLocation)))
    (else
      (Variables|Default|Setcal_z false))))

(event EventOnLanded
  (params (Hit :type Hit%20Result%20Structure%20%28by%20ref%29))
  (bind _returnvalue (Transformation|GetActorLocation))
  (bind _before_z (Variables|Default|Getbefore_z))
  (bind _returnvalue_2 (- _before_z _returnvalue))
  (|CallParentFunction Hit)
  (if (> (.z _returnvalue_2) 1e+02)
    (CallFunction|ShockWave)
    (else
      (Development|PrintString (Utilities|String|ToString(Float) (.z _returnvalue_2))))))

(fn ConstructionScript
  (|CallParentFunction))