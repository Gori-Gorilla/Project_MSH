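; BP_NavProxy is a nav link proxy that makes AI characters jump when they reach its smart link.
; For a BP_AICharacter that is not stopped, it stores the link destination, yaws the character toward it on the flattened XY plane, then calls Jump after a short delay.
; A CalculateJumpVelocity helper computes a gravity-compensated velocity from two points and a duration, but the event graph does not call it.
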(event EventBeginPlay)

(event Collision|EventActorBeginOverlap
  (params (OtherActor :type Actor%20Object%20Reference)))

(event EventTick
  (params (DeltaSeconds :type Float%20%28single-precision%29)))

(event EventSmartLinkReached
  (params (Agent :type Actor%20Object%20Reference) (Destination :type Vector%20%28by%20ref%29 :default "0, 0, 0"))
  (bind (_x _y) (Math|Vector|BreakVector Destination))
  (Development|PrintString "jumplinetest test")
  (bind _asbp_aicharacter (Utilities|Casting|CastToBP_AICharacter Agent))
  (if (not (Variables|/Game/Character/AI/BP_AICharacter.BP_AICharacter_C|GetIsStop _asbp_aicharacter))
    (Variables|/Game/Character/AI/BP_AICharacter.BP_AICharacter_C|SetLinkDestination _asbp_aicharacter Destination)
    (Transformation|SetActorRotation _asbp_aicharacter (Math|Rotator|FindLookatRotation (Math|Vector|MakeVector (.X (Math|Vector|BreakVector (Transformation|GetActorLocation _asbp_aicharacter))) (.Y (Math|Vector|BreakVector (Transformation|GetActorLocation _asbp_aicharacter))) 0.0) (Math|Vector|MakeVector _x _y 0.0)) true)
    (Utilities|FlowControl|Delay 0.2)
    (Character|Jump _asbp_aicharacter)))

(fn ConstructionScript)

(fn CalculateJumpVelocity
  (params (Start%20Vector :type Vector) (Destination%20Vector :type Vector) (Duration :type Float%20%28double-precision%29))
  (bind (_x _y _z) (Math|Vector|BreakVector Start%20Vector))
  (bind (_x_2 _y_2 _z_2) (Math|Vector|BreakVector Destination%20Vector))
  (return (Math|Vector|MakeVector (/ (- _x _x_2) Duration) (/ (- _y _y_2) Duration) (/ (- _z (+ _z_2 (* (Math|Float|Square Duration) -0.5 982.0))) Duration))))