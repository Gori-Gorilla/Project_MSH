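; AI character Blueprint that reacts to overlapping gum and clock-wave actors.
; Touching BP_Gum plays a stepped-on sound, destroys the gum and zeroes walk speed for five seconds before restoring it.
; Touching BP_ClcokWave acts as a time stop: it prints a message, saves the skeletal mesh's linear velocity, disables physics simulation, then re-enables it with that velocity five seconds later.
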(event Collision|EventActorBeginOverlap
  (params (OtherActor :type Actor%20Object%20Reference))
  (bind _charactermovement (Variables|Character|GetCharacterMovement))
  (Utilities|FlowControl|Sequence
    (:then_0
      (bind _asbp_gum (Utilities|Casting|CastToBP_Gum OtherActor))
      (bind _output_get (Variables|Default|Setspeed (Variables|/Script/Engine.CharacterMovementComponent|GetMaxWalkSpeed _charactermovement)))
      (Variables|/Script/Engine.CharacterMovementComponent|SetMaxWalkSpeed _charactermovement 0.0)
      (Audio|PlaySoundatLocation "/Game/sound/Gum_stepped.Gum_stepped" (Transformation|GetActorLocation) "0, 0, 0" 1.0 1.0 0.0 0 0 0 0)
      (Actor|DestroyActor _asbp_gum)
      (Utilities|FlowControl|Delay 5.0)
      (Variables|/Script/Engine.CharacterMovementComponent|SetMaxWalkSpeed _charactermovement _output_get))
    (:then_1
      (Utilities|Casting|CastToBP_ClcokWave OtherActor)
      (Development|PrintString "으아아 타임 슾토픙ㅋ")
      (bind _returnvalue (Physics|GetPhysicsLinearVelocity (Variables|Default|GetSkeletalMesh) "None"))
      (bind _output_get_2 (Variables|Default|SetLinear%20Velocity _returnvalue))
      (Physics|SetSimulatePhysics (Variables|Default|GetSkeletalMesh) false)
      (Utilities|FlowControl|Delay 5.0)
      (Physics|SetSimulatePhysics (Variables|Default|GetSkeletalMesh) true)
      (Physics|SetPhysicsLinearVelocity (Variables|Default|GetSkeletalMesh) _output_get_2 false "None"))))

(fn ConstructionScript)